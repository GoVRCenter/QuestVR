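; PC_Default is a player controller that spawns and possesses a motion controller pawn when play begins.
; A custom event picks a random PlayerStart in the level and spawns the MotionControllerPawn at its transform, owned by the controller.
; Spawning adjusts position to avoid collisions but always spawns, then the controller possesses the new pawn.
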(event `self.ReceiveBeginPlay`
  ;[1 1 1] Begin Play
  (`self.SpawnAndPossessPawn`))

(event `SpawnAndPossessPawn`
  ;[1 1 1] Spawn and Possess
  (bind _outactors (`GameplayStatics.GetAllActorsOfClass` "/Script/Engine.PlayerStart"))
  (bind _returnvalue (`|SpawnActorFromClass` "/Game/VirtualRealityBP/Blueprints/MotionControllerPawn.MotionControllerPawn_C" (`self.GetTransform` (`|GetArrayItem` _outactors (`KismetMathLibrary.RandomIntegerInRange` 0 (- (`KismetArrayLibrary.Array_Length` _outactors) 1)))) "AdjustIfPossibleButAlwaysSpawn" "OverrideRootScale" self null))
  (`self.Possess` _returnvalue))

(fn `UserConstructionScript`)